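; BP_GDCharacterHero is the hero character Blueprint for Aura, handling player movement, look input and facing targets for motion warping.
; Enhanced Input drives movement along the actor's forward (X) and right (Y) vectors, and controller yaw and pitch, with pitch inverted.
; UpdateFacingTarget passes a location to the Motion Warping component as the "FacingTarget" warp target, which lets warped animations turn toward it.
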(event `CombatInterface.UpdateFacingTarget`
  (params (Location :type "Vector Structure"))
  (`MotionWarpingComponent.AddOrUpdateWarpTargetFromLocation` (`self.MotionWarping`) "FacingTarget" Location))

(event `EnhancedInput|/Game/GDContent/Input/IA_Move`
  (params (ActionValue :type "Vector2D Structure") (ElapsedSeconds :type "Float (double-precision)") (TriggeredSeconds :type "Float (double-precision)") (InputAction :type "InputAction Object Reference" :default "/Game/GDContent/Input/IA_Move.IA_Move"))
  (:`Triggered`
    (`self.AddMovementInput` (`self.GetActorForwardVector`) ActionValue_X)
    (`self.AddMovementInput` (`self.GetActorRightVector`) ActionValue_Y)))

(event `EnhancedInput|/Game/GDContent/Input/IA_Look`
  (params (ActionValue :type "Vector2D Structure") (ElapsedSeconds :type "Float (double-precision)") (TriggeredSeconds :type "Float (double-precision)") (InputAction :type "InputAction Object Reference" :default "/Game/GDContent/Input/IA_Look.IA_Look"))
  (:`Triggered`
    (`self.AddControllerYawInput` ActionValue_X)
    (`self.AddControllerPitchInput` (* ActionValue_Y -1.0))))

(fn `UserConstructionScript`)