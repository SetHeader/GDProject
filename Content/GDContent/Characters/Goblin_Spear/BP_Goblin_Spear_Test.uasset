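; Test variant of the spear goblin character that checks attack montage events against the spear tip position.
; Shortly after BeginPlay it plays the spear attack montage on its mesh, then starts listening for the Montage.Attack.1 gameplay event on the actor.
; Each received event draws a brief debug sphere at the weapon component's TipSocket, showing where the tip is at that moment.
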(event `self.ReceiveBeginPlay`
  (`parent.ReceiveBeginPlay`)
  (`KismetSystemLibrary.Delay` 3.0)
  (`KismetSystemLibrary.PrintString` "play")
  (`|PlayMontage` (`self.Mesh`) "/Game/GDContent/Animations/Goblin/AM_Spear_Attack.AM_Spear_Attack"
    (:`then`
      (`AbilityAsync_WaitGameplayEvent.WaitGameplayEventToActor` null (struct :`TagName` "Montage.Attack.1")
        (:`EventReceived`
          (`KismetSystemLibrary.DrawDebugSphere` (`SceneComponent.GetSocketLocation` (`self.WeaponComponent`) "TipSocket") 8.0 12 (struct :`R` 1.0 :`G` 1.0 :`B` 1.0 :`A` 1.0) 2.0))))))

(fn `UserConstructionScript`
  (`parent.UserConstructionScript`))