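; Gameplay ability for Arcane Shards: the player aims with a magic circle, then shards erupt around the clicked point.
; A press hides the circle, turns the caster, plays the cast montage and gets level-scaled, capped ground points from a BP_PointCollection.
; A montage event commits the ability and starts a looping timer that spawns shards sequentially.
; Each shard fires a GameplayCue and applies radial damage with outward knockback until all points are used.
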(event `self.K2_ActivateAbility`
  (`|ExecutionSequence`
    (:`then_0`
      (bind _asbp_gdplayer_controller (cast `/Game/GDContent/Blueprints/BP_GDPlayerController` (`GameplayStatics.GetPlayerController` 0)))
      (set `self.As BP GDPlayer Controller` _asbp_gdplayer_controller))
    (:`then_1`
      (`GDPlayerController.ShowMagicCircle` (`self.As BP GDPlayer Controller`) null)
      (`AbilityTask_WaitInputPress.WaitInputPress` false
        (:`OnPress`
          (`|ExecutionSequence`
            (:`then_0`
              ;[1 1 1] 隐藏魔法阵、让角色旋转至鼠标点击方向
              (`GDPlayerController.HideMagicCircle` (`self.As BP GDPlayer Controller`))
              (bind (_asynctaskproxy _datadatahandle) (`TargetDataUnderMouse.CreateTargetDataUnderMouse`)
                (:`OnValidDataDelegate`
                  (set `self.MouseHitPoint` (`.ImpactPoint` (`GameplayStatics.BreakHitResult` (`AbilitySystemBlueprintLibrary.GetHitResultFromTargetData` _datadatahandle)))))))
            (:`then_1`
              (message `CombatInterface.UpdateFacingTarget` (`self.GetAvatarActorFromActorInfo`) (`self.MouseHitPoint`))
              (`AbilityTask_PlayMontageAndWait.CreatePlayMontageAndWaitProxy` "None" "/Game/GDContent/Animations/Aura/AM_Cast_Shards.AM_Cast_Shards"))
            (:`then_2`
              ;[1 1 1] 获取生成碎片的位置
              (bind _returnvalue (`|SpawnActorFromClass` "/Game/GDContent/Blueprints/Actor/PointCollection/BP_PointCollection.BP_PointCollection_C" (`KismetMathLibrary.MakeTransform` (`self.MouseHitPoint`)) "Undefined" "MultiplyWithRoot" null null))
              (bind _output_get (set `self.PointCollection` _returnvalue))
              (set `self.ShardPoints` (`PointCollection.GetGroundPoints` _output_get (`self.MouseHitPoint`) (`KismetMathLibrary.Min` (`self.MaxShardsCount`) (`self.GetAbilityLevel`)) (`KismetMathLibrary.RandomFloatInRange` 0.0 360.0))))
            (:`then_3`
              (`AbilityTask_WaitGameplayEvent.WaitGameplayEvent` (struct :`TagName` "Event.Montage.ArcaneShards") null true
                (:`EventReceived`
                  (`self.K2_CommitAbility`)
                  (set `self.ShardIdx` 0)
                  (bind _returnvalue_2 (`KismetSystemLibrary.K2_SetTimerDelegate` (delegate `SpawnShard`) (`self.SpawnShardTime`) true))
                  (set `self.SpawnShardTimerHandler` _returnvalue_2)
                  (`self.GenerateShardAndApplyEffect` (`|GetArrayItem` (`self.ShardPoints`) (`self.ShardIdx`)))
                  (`/Engine/EditorBlueprintResources/StandardMacros.IncrementInt` (`self.ShardIdx`)
                    (:`  `
                      (`self.IsShardIdxValid`
                        (:`false`
                          (`self.CleanAndEndAbility`))))))))))))))

(event `SpawnShard`
  ;[1 1 1] 定时生成地刺
  (`self.IsShardIdxValid`
    (:`true`
      (`|ExecutionSequence`
        (:`then_0`
          (`self.GenerateShardAndApplyEffect` (`|GetArrayItem` (`self.ShardPoints`) (`self.ShardIdx`))))
        (:`then_1`
          (`/Engine/EditorBlueprintResources/StandardMacros.IncrementInt` (`self.ShardIdx`)
            (:`  `
              (`self.IsShardIdxValid`
                (:`false`
                  (`self.CleanAndEndAbility`))))))))
    (:`false`
      (`self.CleanAndEndAbility`))))

(fn `CleanAndEndAbility`
  (`KismetSystemLibrary.K2_ClearAndInvalidateTimerHandle` (`self.SpawnShardTimerHandler`))
  (`self.K2_RemoveGameplayCue` (struct :`TagName` "GameplayCue.ArcaneShards"))
  (`self.K2_EndAbility`))

(fn `GenerateShardAndApplyEffect`
  (params (ShardPoint :type "SceneComponent Object Reference"))
  (locals (ShardPointLocation :type "Vector Structure" :default (0.0 0.0 0.0)))
  (bind _returnvalue (`self.GetAvatarActorFromActorInfo`))
  (set `local.ShardPointLocation` (`SceneComponent.K2_GetComponentLocation` ShardPoint))
  (`|ExecutionSequence`
    (:`then_0`
      (`self.K2_ExecuteGameplayCueWithParams` (struct :`TagName` "GameplayCue.ArcaneShards") (`AbilitySystemBlueprintLibrary.MakeGameplayCueParameters` 0.0 0.0 (struct) (struct) (struct) (struct) (struct) (`local.ShardPointLocation`))))
    (:`then_1`
      (bind _outoverlappingactors (`GDAbilitySystemLibrary.GetLivePlayersWithInRadius` _returnvalue (`|MakeArray` _returnvalue) (`self.RadialDamageOuterRadius`) (`local.ShardPointLocation`)))
      (for _array_element _outoverlappingactors
        (bind _returnvalue_2 (- (`Actor.K2_GetActorLocation` _array_element) (`local.ShardPointLocation`)))
        (`GDAbilitySystemLibrary.ApplyDamageEffect` (`self.MakeDamageEffectParamsFromClassDefaults` _array_element (`local.ShardPointLocation`) true _returnvalue_2 true _returnvalue_2 true 20.0))))))