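; Enemy ranged attack gameplay ability that fires an arced projectile at the avatar's combat target.
; After committing, it picks a random tagged montage, turns to the target and plays it while waiting for that montage's gameplay event.
; The event spawns the projectile from the tagged socket with a pitch override, then ends the ability without stopping the montage.
; An ApplyDamage radius-check function with debug drawing is defined but never called here.
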(event `self.K2_ActivateAbility`
  (bind _returnvalue (`self.GetAvatarActorFromActorInfo`))
  (bind _returnvalue_2 (`self.K2_CommitAbility`))
  (if _returnvalue_2
    (bind _returnvalue_3 (message `EnemyInterface.GetCombatTarget` _returnvalue))
    (`/Engine/EditorBlueprintResources/StandardMacros.IsValid` _returnvalue_3
      (:`Is Valid`
        (bind _ascombat_interface (cast `CombatInterface` _returnvalue)
          (:`then`
            (bind (_output _found) (`self.Find Random Attack Montage` _ascombat_interface))
            (if _found
              (bind _returnvalue_4 (`Actor.K2_GetActorLocation` _returnvalue_3))
              (`CombatInterface.UpdateFacingTarget` _ascombat_interface _returnvalue_4)
              (bind (_montage _montagetag _sockettag) (break `TaggedMontage` _output))
              (`AbilityTask_WaitGameplayEvent.WaitGameplayEvent` _montagetag null
                (:`then`
                  (`AbilityTask_PlayMontageAndWait.CreatePlayMontageAndWaitProxy` "None" _montage 1.0 "None" false
                    (:`OnCompleted`
                      _)
                    (:`OnInterrupted`
                      _)
                    (:`OnCancelled`
                      _)))
                (:`EventReceived`
                  (`self.SpawnProjectile` _returnvalue_4 _sockettag 40.0 true null)))))
          (:`CastFailed`
            _)))
      (:`Is Not Valid`
        _))
    (`self.K2_EndAbility`)
    (else
      (`self.K2_EndAbility`))))

(fn `Apply Damage`
  (params (CombatInterface :type "CombatInterface Interface") (MontageTag :type "GameplayTag Structure (by ref)"))
  (bind _returnvalue (`CombatInterface.GetCombatSocketLocation` CombatInterface MontageTag))
  (`KismetSystemLibrary.DrawDebugSphere` _returnvalue 8.0 12 (struct :`R` 1.0 :`G` 0.032104 :`A` 1.0) 3.0)
  (bind _outoverlappingactors (`GDAbilitySystemLibrary.GetLivePlayersWithInRadius` (`self.GetAvatarActorFromActorInfo`) (`|MakeArray` null :!type "Actor Object Reference") 32.0 _returnvalue))
  (for _array_element _outoverlappingactors
    (if (!= _array_element (`self.GetAvatarActorFromActorInfo`))
      (`self.CauseDamage` _array_element)))
  (return))

(fn `Find Random Attack Montage`
  (params (CombatInterface :type "CombatInterface Interface"))
  (returns (Output :type "TaggedMontage Structure") (Found :type Boolean))
  (locals (TaggedMontages :type "Array of TaggedMontage Structure"))
  (bind _returnvalue (`CombatInterface.GetTaggedMontages` CombatInterface))
  (set `local.TaggedMontages` _returnvalue)
  (if (`KismetArrayLibrary.Array_IsNotEmpty` (`local.TaggedMontages`))
    (return (`|GetArrayItem` (`local.TaggedMontages`) (`KismetMathLibrary.RandomIntegerInRange` 0 (- (`KismetArrayLibrary.Array_Length` (`local.TaggedMontages`)) 1))) true)
    (else
      (return (struct) false))))