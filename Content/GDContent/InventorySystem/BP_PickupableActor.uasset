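; BP_PickupableActor is an inventory-system actor that animates its mesh as a spinning, floating item.
; Each tick it adds yaw scaled by RotationsPerSecond (using 365 degrees per turn) and sets relative Z from a smoothing helper.
; The helper maps C_Smooth_Up_Down over FloatingPeriod between negative and positive MaxFloatingHeight, the negative bound being computed at BeginPlay.
; The graph contains no pickup logic.
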(event `self.ReceiveBeginPlay`
  (set `self.NagativeMaxFloatingHeight` (* (`self.MaxFloatingHeight`) -1.0)))

(event `self.ReceiveTick`
  (params (DeltaSeconds :type "Float (single-precision)"))
  (`SceneComponent.K2_AddRelativeRotation` (`self.StaticMeshComponent`) (`KismetMathLibrary.MakeRotator` 0.0 0.0 (* DeltaSeconds (`self.RotationsPerSecond`) 365.0)) false false)
  (bind _outvalue (`/Game/GDContent/Tools/BP_FunctionTools.SmoothlyGetMappedCurveValue` (`self.ElapsedTime`) "/Game/GDContent/Assets/Curve/C_Smooth_Up_Down.C_Smooth_Up_Down" DeltaSeconds 1.0 (`self.FloatingPeriod`) 0.0 1.0 (`self.NagativeMaxFloatingHeight`) (`self.MaxFloatingHeight`)))
  (`SceneComponent.K2_SetRelativeLocation` (`self.StaticMeshComponent`) (`KismetMathLibrary.MakeVector` 0.0 0.0 _outvalue) false false))

(fn `UserConstructionScript`)