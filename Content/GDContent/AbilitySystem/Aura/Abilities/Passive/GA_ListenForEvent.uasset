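; Passive gameplay ability for Aura that turns incoming Attribute gameplay events into attribute effects on its owner.
; On activation it waits for events matching the Attribute tag hierarchy, then builds a spec from a configurable effect class.
; It sets SetByCaller magnitudes for every default tag, using the event magnitude for the matching tag and zero for the rest.
; The spec is then applied to the owner.
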(event `self.K2_ActivateAbility`
  (bind ((`EventTag` _eventtag) (`EventMagnitude` _eventmagnitude)) (break `GameplayEventData` (`self.EventPayload`)))
  (bind (_asynctaskproxy _payload) (`AbilityTask_WaitGameplayEvent.WaitGameplayEvent` (struct :`TagName` "Attribute") null false false)
    (:`EventReceived`
      (set `self.EventPayload` _payload)
      (set `self.GESpec` (`self.MakeOutgoingGameplayEffectSpec` (`self.Gameplay Effect Class`)))
      (for _array_element (`self.DefaultTags`)
        (if (== _array_element _eventtag)
          (`AbilitySystemBlueprintLibrary.AssignTagSetByCallerMagnitude` (`self.GESpec`) _eventtag _eventmagnitude)
          (else
            (`AbilitySystemBlueprintLibrary.AssignTagSetByCallerMagnitude` (`self.GESpec`) _array_element))))
      (`self.K2_ApplyGameplayEffectSpecToOwner` (`self.GESpec`)))))