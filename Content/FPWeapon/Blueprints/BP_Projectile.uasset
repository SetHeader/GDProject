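; BP_Projectile is a weapon projectile that applies a Gameplay Ability System effect to characters it overlaps, ignoring its owner.
; On sphere overlap, it gets the ability system components of the hit GDCharacterBase and the instigator.
; A Visibility trace from the instigator to the projectile supplies a hit result for the outgoing effect spec's context.
; The spec is applied to the target only if that trace hits something.
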(event `self.Sphere.OnComponentBeginOverlap`
  (params (OverlappedComponent :type "PrimitiveComponent Object Reference") (OtherActor :type "Actor Object Reference") (OtherComp :type "PrimitiveComponent Object Reference") (OtherBodyIndex :type Integer) (bFromSweep :type Boolean) (SweepResult :type "HitResult Structure (by ref)"))
  (`self.OnBeginOverlap` OtherActor))

(fn `OnBeginOverlap`
  (params (OtherActor :type "Object Object Reference"))
  (locals (SourceASC :type "AbilitySystemComponent Object Reference") (TargetASC :type "AbilitySystemComponent Object Reference") (CachedGE :type "GameplayEffectSpecHandle Structure") (CachedOutHit :type "HitResult Structure"))
  (if (not (== OtherActor (`self.GetOwner`)))
    (bind _asgdcharacter_base (cast `GDCharacterBase` OtherActor))
    (set `local.TargetASC` (`AbilitySystemBlueprintLibrary.GetAbilitySystemComponent` _asgdcharacter_base))
    (bind _asgdcharacter_base_2 (cast `GDCharacterBase` (`self.GetInstigator`)))
    (set `local.SourceASC` (`AbilitySystemBlueprintLibrary.GetAbilitySystemComponent` _asgdcharacter_base_2))
    (bind (_outhit _returnvalue) (`KismetSystemLibrary.LineTraceSingle` (`self.K2_GetActorLocation` _asgdcharacter_base_2) (`self.K2_GetActorLocation`) "TraceTypeQuery1"))
    (if _returnvalue
      (set `local.CachedOutHit` _outhit)
      (bind _output_get (set `local.CachedGE` (`AbilitySystemComponent.MakeOutgoingSpec` :`self` (`local.SourceASC`) :`GameplayEffectClass` (`self.GameplayEffect`) :`Level` (`self.Level`))))
      (bind _returnvalue_2 (`AbilitySystemBlueprintLibrary.GetEffectContext` _output_get))
      (`AbilitySystemBlueprintLibrary.EffectContextAddHitResult` _returnvalue_2 (`local.CachedOutHit`))
      (`AbilitySystemComponent.BP_ApplyGameplayEffectSpecToSelf` (`local.TargetASC`) _output_get))))

(fn `UserConstructionScript`)