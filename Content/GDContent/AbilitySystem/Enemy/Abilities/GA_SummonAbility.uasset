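; Enemy gameplay ability for summoning, which so far shows only ground effects and debug markers, with no actors spawned.
; On activation it caches the result of GetSpawnLocations, shuffles it and plays the ground-summon Niagara effect at every point at once.
; After a short delay, a second loop draws a debug sphere at each point, with a Delay in the loop body.
; The graph never calls EndAbility.
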(event `self.K2_ActivateAbility`
  (bind _returnvalue (`self.GetSpawnLocations`))
  (bind _output_get (set `self.SpawnLocations` _returnvalue))
  (`KismetArrayLibrary.Array_Shuffle` _output_get)
  (for _array_element (`self.SpawnLocations`)
    (`NiagaraFunctionLibrary.SpawnSystemAtLocation` "/Game/Assets/Effects/Combat/NS_GroundSummon.NS_GroundSummon" _array_element (struct) (1.0 1.0 1.0) true true "AutoRelease"))
  (`KismetSystemLibrary.Delay` 1.0)
  (for _array_element_2 (`self.SpawnLocations`)
    (`KismetSystemLibrary.DrawDebugSphere` _array_element_2 16.0 8 (struct :`R` 1.0 :`A` 1.0) 3.0)
    (`KismetSystemLibrary.Delay` 0.2)))