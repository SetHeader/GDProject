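; Fire bolt gameplay ability that casts a projectile toward the point under the mouse cursor.
; Once the ability commits, a target data task supplies the hit result and the avatar turns toward it through CombatInterface.
; The cast montage plays, and its gameplay event times the projectile spawn from the weapon socket toward the impact point before the ability ends.
; A failed commit ends the ability immediately.
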(event `self.K2_ActivateAbility`
  (bind _returnvalue (`self.K2_CommitAbility`))
  (if _returnvalue
    (bind (_asynctaskproxy _datadatahandle) (`TargetDataUnderMouse.CreateTargetDataUnderMouse`)
      (:`OnValidDataDelegate`
        (bind _output_get (set `self.HitResult` (`AbilitySystemBlueprintLibrary.GetHitResultFromTargetData` _datadatahandle)))
        (bind _ascombat_interface (cast `CombatInterface` (`self.GetAvatarActorFromActorInfo`)))
        (`CombatInterface.UpdateFacingTarget` _ascombat_interface (`.Location` (`GameplayStatics.BreakHitResult` _output_get)))
        (`AbilityTask_PlayMontageAndWait.CreatePlayMontageAndWaitProxy` "None" "/Game/GDContent/Animations/Aura/AM_Cast_FireBolt.AM_Cast_FireBolt" 1.0 "None" false
          (:`then`
            (`AbilityTask_WaitGameplayEvent.WaitGameplayEvent` (struct :`TagName` "Event.Montage.FireBolt") null
              (:`EventReceived`
                (`self.SpawnProjectile` (`.ImpactPoint` (`GameplayStatics.BreakHitResult` (`self.HitResult`))) (`BlueprintGameplayTagLibrary.MakeLiteralGameplayTag` (struct :`TagName` "CombatSocket.Weapon")) 0.0 false null)
                (`self.K2_EndAbility`)))))))
    (else
      (`self.K2_EndAbility`))))