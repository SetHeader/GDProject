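; BP_MeleeAttack is a Gameplay Ability for a spear melee attack against the avatar's combat target.
; After committing, it gets the target, turns the avatar to face it through CombatInterface and plays the spear attack montage.
; On authority, it waits for the melee montage event, draws a debug sphere at the combat socket and ends the ability.
; No damage is applied yet.
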(event `self.K2_ActivateAbility`
  (bind _returnvalue (`self.GetAvatarActorFromActorInfo`))
  (bind _returnvalue_2 (`self.K2_CommitAbility`))
  (if _returnvalue_2
    (bind _returnvalue_3 (message `EnemyInterface.GetCombatTarget` _returnvalue))
    (`/Engine/EditorBlueprintResources/StandardMacros.IsValid` _returnvalue_3
      (:`Is Valid`
        (bind _ascombat_interface (cast `CombatInterface` _returnvalue)
          (:`then`
            (`CombatInterface.UpdateFacingTarget` _ascombat_interface (`Actor.K2_GetActorLocation` _returnvalue_3))
            (`AbilityTask_PlayMontageAndWait.CreatePlayMontageAndWaitProxy` "None" "/Game/GDContent/Animations/Goblin/AM_Spear_Attack.AM_Spear_Attack"
              (:`then`
                (`self.K2_HasAuthority`
                  (:`True`
                    (`AbilityTask_WaitGameplayEvent.WaitGameplayEvent` (struct :`TagName` "Event.Montage.Melee") null
                      (:`EventReceived`
                        (bind _returnvalue_4 (`CombatInterface.GetCombatSocketLocation` _ascombat_interface))
                        (`KismetSystemLibrary.DrawDebugSphere` _returnvalue_4 16.0 12 (struct :`R` 1.0 :`A` 1.0) 3.0))))))))
          (:`CastFailed`
            _)))
      (:`Is Not Valid`
        _))
    (`self.K2_EndAbility`)
    (else
      (`self.K2_EndAbility`))))