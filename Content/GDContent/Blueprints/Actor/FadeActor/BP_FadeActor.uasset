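; BP_FadeActor is an actor meant to fade its static mesh when something overlaps it.
; BeginPlay creates a dynamic material instance with Fade at 1, but assigns the base FadeMaterial to the mesh rather than that instance.
; Begin overlap plays FadeTimeline and end overlap reverses it, with timeline updates writing the instance's Fade parameter.
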(event `self.ReceiveBeginPlay`
  (bind _returnvalue (`KismetMaterialLibrary.CreateDynamicMaterialInstance` (`self.FadeMaterial`)))
  (bind _output_get (set `self.FadeMaterialDynamic` _returnvalue))
  (`MaterialInstanceDynamic.SetScalarParameterValue` _output_get "Fade" 1.0)
  (`PrimitiveComponent.SetMaterial` (`self.StaticMesh`) 0 (`self.FadeMaterial`)))

(event `/Game/GDContent/Blueprints/Actor/FadeActor/BI_FadeInterface.FadeIn`
  (bind (_direction _fadein) (`Timeline|FadeTimeline` :!label _label)
    (:`Update`
      (`MaterialInstanceDynamic.SetScalarParameterValue` (`self.FadeMaterialDynamic`) "Fade" _fadein))))

(event `/Game/GDContent/Blueprints/Actor/FadeActor/BI_FadeInterface.FadeOut`
  (goto _label :!via `Reverse`))

(event `self.StaticMesh.OnComponentBeginOverlap`
  (params (OverlappedComponent :type "PrimitiveComponent Object Reference") (OtherActor :type "Actor Object Reference") (OtherComp :type "PrimitiveComponent Object Reference") (OtherBodyIndex :type Integer) (bFromSweep :type Boolean) (SweepResult :type "HitResult Structure (by ref)"))
  (`/Game/GDContent/Blueprints/Actor/FadeActor/BI_FadeInterface.FadeIn`))

(event `self.StaticMesh.OnComponentEndOverlap`
  (params (OverlappedComponent :type "PrimitiveComponent Object Reference") (OtherActor :type "Actor Object Reference") (OtherComp :type "PrimitiveComponent Object Reference") (OtherBodyIndex :type Integer))
  (`/Game/GDContent/Blueprints/Actor/FadeActor/BI_FadeInterface.FadeOut`))

(fn `UserConstructionScript`)