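; Minion AI character Blueprint that keeps an info widget in sync with its health, mana and stamina.
; On BeginPlay, only instances without authority bind to the GDASBase change delegates for those attributes and their maximums.
; Each handler writes the new value into the Info struct of the UI_Info widget from the WidgetInfo component, then calls UpdateUI.
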(event `self.ReceiveBeginPlay`
  (bind _returnvalue (`self.GetGDASBase`))
  (`/Engine/EditorBlueprintResources/ActorMacros.Switch Has Authority`
    (:`Remote`
      (add `GDAttributeSetBase.OnHealthChangedDelegate` _returnvalue (delegate `OnHealthChangedDelegate_Event`))
      (add `GDAttributeSetBase.OnMaxHealthChangedDelegate` _returnvalue (delegate `OnMaxHealthChangedDelegate_Event`))
      (add `GDAttributeSetBase.OnManaChangedDelegate` _returnvalue (delegate `OnManaChangedDelegate_Event`))
      (add `GDAttributeSetBase.OnMaxManaChangedDelegate` _returnvalue (delegate `OnMaxManaChangedDelegate_Event`))
      (add `GDAttributeSetBase.OnStaminaChangedDelegate` _returnvalue (delegate `OnStaminaChangedDelegate_Event`))
      (add `GDAttributeSetBase.OnMaxStaminaChangedDelegate` _returnvalue (delegate `OnMaxStaminaChangedDelegate_Event`)))))

(event `OnHealthChangedDelegate_Event`
  (params (NewValue :type "Float (single-precision)") (OldValue :type "Float (single-precision)"))
  (bind _asui_info (`self.GetInfoWidget`))
  (setmembers `GDASBase` :`StructRef` (`/Game/GDContent/UI/UI_Info.Info` _asui_info) :`Health` NewValue)
  (`/Game/GDContent/UI/UI_Info.UpdateUI` _asui_info))

(event `OnMaxHealthChangedDelegate_Event`
  (params (NewValue :type "Float (single-precision)") (OldValue :type "Float (single-precision)"))
  (bind _asui_info (`self.GetInfoWidget`))
  (setmembers `GDASBase` :`StructRef` (`/Game/GDContent/UI/UI_Info.Info` _asui_info) :`MaxHealth` NewValue)
  (`/Game/GDContent/UI/UI_Info.UpdateUI` _asui_info))

(event `OnManaChangedDelegate_Event`
  (params (NewValue :type "Float (single-precision)") (OldValue :type "Float (single-precision)"))
  (bind _asui_info (`self.GetInfoWidget`))
  (setmembers `GDASBase` :`StructRef` (`/Game/GDContent/UI/UI_Info.Info` _asui_info) :`Mana` NewValue)
  (`/Game/GDContent/UI/UI_Info.UpdateUI` _asui_info))

(event `OnMaxManaChangedDelegate_Event`
  (params (NewValue :type "Float (single-precision)") (OldValue :type "Float (single-precision)"))
  (bind _asui_info (`self.GetInfoWidget`))
  (setmembers `GDASBase` :`StructRef` (`/Game/GDContent/UI/UI_Info.Info` _asui_info) :`MaxMana` NewValue)
  (`/Game/GDContent/UI/UI_Info.UpdateUI` _asui_info))

(event `OnStaminaChangedDelegate_Event`
  (params (NewValue :type "Float (single-precision)") (OldValue :type "Float (single-precision)"))
  (bind _asui_info (`self.GetInfoWidget`))
  (setmembers `GDASBase` :`StructRef` (`/Game/GDContent/UI/UI_Info.Info` _asui_info) :`Stamina` NewValue)
  (`/Game/GDContent/UI/UI_Info.UpdateUI` _asui_info))

(event `OnMaxStaminaChangedDelegate_Event`
  (params (NewValue :type "Float (single-precision)") (OldValue :type "Float (single-precision)"))
  (bind _asui_info (`self.GetInfoWidget`))
  (setmembers `GDASBase` :`StructRef` (`/Game/GDContent/UI/UI_Info.Info` _asui_info) :`MaxStamina` NewValue)
  (`/Game/GDContent/UI/UI_Info.UpdateUI` _asui_info))

(fn `GetInfoWidget`
  (returns (`AsUI Info` :type "/Game/GDContent/UI/UI_Info Object Reference"))
  (bind _asui_info (cast `/Game/GDContent/UI/UI_Info` (`WidgetComponent.GetWidget` (`self.WidgetInfo`))))
  (return _asui_info))

(fn `UserConstructionScript`)