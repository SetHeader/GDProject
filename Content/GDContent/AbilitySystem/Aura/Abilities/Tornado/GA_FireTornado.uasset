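; GA_FireTornado is a gameplay ability that casts a fire tornado projectile toward the point under the mouse cursor.
; On activation it takes the hit location from target data, turns the avatar to face it and plays the cast montage.
; The montage's gameplay event triggers the cost and cooldown commit, then spawns the projectile from the weapon socket and ends the ability.
; A failed commit leaves the ability without an EndAbility call.
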(event `self.K2_ActivateAbility`
  (bind (_asynctaskproxy _datadatahandle) (`TargetDataUnderMouse.CreateTargetDataUnderMouse`)
    (:`OnValidDataDelegate`
      (bind _output_get (set `self.TargetLocation` (`.Location` (`GameplayStatics.BreakHitResult` (`AbilitySystemBlueprintLibrary.GetHitResultFromTargetData` _datadatahandle)))))
      (message `CombatInterface.UpdateFacingTarget` (`self.GetAvatarActorFromActorInfo`) _output_get)
      (`AbilityTask_PlayMontageAndWait.CreatePlayMontageAndWaitProxy` "None" "/Game/GDContent/Animations/Aura/AM_Cast_FireTornado.AM_Cast_FireTornado"
        (:`then`
          (`AbilityTask_WaitGameplayEvent.WaitGameplayEvent` (struct :`TagName` "Event.Montage.FireTornado") null
            (:`EventReceived`
              (bind _returnvalue (`self.K2_CommitAbility`))
              (if _returnvalue
                (`self.SpawnProjectile` (`self.TargetLocation`) (`BlueprintGameplayTagLibrary.MakeLiteralGameplayTag` (struct :`TagName` "CombatSocket.Weapon")) 0.0 false null)
                (`self.K2_EndAbility`)))))))))