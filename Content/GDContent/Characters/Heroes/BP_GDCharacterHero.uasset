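; Hero character Blueprint that turns Enhanced Input into movement, camera look and Gameplay Ability System skill activation.
; Move input drives movement along the actor's forward and right vectors, and look input drives controller yaw and inverted pitch.
; Fire, FireBall and IceBall inputs each try to activate abilities by gameplay tag.
; An UpdateFacingTarget event feeds a location into Motion Warping as the FacingTarget warp target.
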(event `CombatInterface.UpdateFacingTarget`
  (params (Location :type "Vector Structure"))
  (`MotionWarpingComponent.AddOrUpdateWarpTargetFromLocation` (`self.MotionWarping`) "FacingTarget" Location))

(event `EnhancedInput|/Game/GDContent/Input/IA_Move`
  (params (ActionValue :type "Vector2D Structure") (ElapsedSeconds :type "Float (double-precision)") (TriggeredSeconds :type "Float (double-precision)") (InputAction :type "InputAction Object Reference" :default "/Game/GDContent/Input/IA_Move.IA_Move"))
  (:`Triggered`
    (`self.AddMovementInput` (`self.GetActorForwardVector`) ActionValue_X)
    (`self.AddMovementInput` (`self.GetActorRightVector`) ActionValue_Y)))

(event `EnhancedInput|/Game/GDContent/Input/IA_Look`
  (params (ActionValue :type "Vector2D Structure") (ElapsedSeconds :type "Float (double-precision)") (TriggeredSeconds :type "Float (double-precision)") (InputAction :type "InputAction Object Reference" :default "/Game/GDContent/Input/IA_Look.IA_Look"))
  (:`Triggered`
    (`self.AddControllerYawInput` ActionValue_X)
    (`self.AddControllerPitchInput` (* ActionValue_Y -1.0))))

(event `EnhancedInput|/Game/GDContent/Input/IA_Fire`
  (params (ActionValue :type Boolean) (ElapsedSeconds :type "Float (double-precision)") (TriggeredSeconds :type "Float (double-precision)") (InputAction :type "InputAction Object Reference" :default "/Game/GDContent/Input/IA_Fire.IA_Fire"))
  (:`Triggered`
    (`AbilitySystemComponent.TryActivateAbilitiesByTag` (`AbilitySystemBlueprintLibrary.GetAbilitySystemComponent` null) (`BlueprintGameplayTagLibrary.MakeGameplayTagContainerFromTag` (struct :`TagName` "Ability.Skill.Fire")) true)))

(event `EnhancedInput|/Game/GDContent/Input/IA_FireBall`
  (params (ActionValue :type Boolean) (ElapsedSeconds :type "Float (double-precision)") (TriggeredSeconds :type "Float (double-precision)") (InputAction :type "InputAction Object Reference" :default "/Game/GDContent/Input/IA_FireBall.IA_FireBall"))
  (:`Triggered`
    (`AbilitySystemComponent.TryActivateAbilitiesByTag` (`AbilitySystemBlueprintLibrary.GetAbilitySystemComponent` null) (`BlueprintGameplayTagLibrary.MakeGameplayTagContainerFromTag` (struct :`TagName` "Ability.Skill.FireBall")) true)))

(event `EnhancedInput|/Game/GDContent/Input/IA_IceBall`
  (params (ActionValue :type Boolean) (ElapsedSeconds :type "Float (double-precision)") (TriggeredSeconds :type "Float (double-precision)") (InputAction :type "InputAction Object Reference" :default "/Game/GDContent/Input/IA_IceBall.IA_IceBall"))
  (:`Triggered`
    (`AbilitySystemComponent.TryActivateAbilitiesByTag` (`AbilitySystemBlueprintLibrary.GetAbilitySystemComponent` null) (`BlueprintGameplayTagLibrary.MakeGameplayTagContainerFromTag` (struct :`TagName` "Ability.Skill.IceBall")) true)))

(fn `UserConstructionScript`)