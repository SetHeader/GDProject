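; Gameplay ability that fires an ice ball projectile from the player hero's weapon.
; On activation it resolves the hero pawn through the owning PlayerState, then commits the ability.
; A successful commit spawns BP_Projectile_IceBall at the weapon's Muzzle socket along the control rotation, with the hero as owner and instigator.
; The ability ends immediately on every path, including failed casts or commit.
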(event `self.K2_ActivateAbility`
  (bind _returnvalue_owneractor (break `GameplayAbilityActorInfo` (`self.GetActorInfo`)))
  (bind _asbp_gdplayer_state (cast `/Game/GDContent/Blueprints/BP_GDPlayerState` _returnvalue_owneractor)
    (:`then`
      (bind _asbp_gdcharacter_hero (cast `/Game/GDContent/Characters/Heroes/BP_GDCharacterHero` (`PlayerState.GetPawn` _asbp_gdplayer_state))
        (:`then`
          (bind _returnvalue (`self.K2_CommitAbility`))
          (if _returnvalue
            (`|SpawnActorFromClass` "/Game/FPWeapon/Blueprints/BP_Projectile_IceBall.BP_Projectile_IceBall_C" (`KismetMathLibrary.MakeTransform` (`SceneComponent.GetSocketLocation` (`GDCharacterBase.WeaponComponent` _asbp_gdcharacter_hero) "Muzzle") (`Pawn.GetControlRotation` _asbp_gdcharacter_hero)) "AlwaysSpawn" "OverrideRootScale" _asbp_gdcharacter_hero _asbp_gdcharacter_hero))
          (`self.K2_EndAbility`))
        (:`CastFailed`
          (`self.K2_EndAbility` :!label _label))))
    (:`CastFailed`
      (goto _label))))