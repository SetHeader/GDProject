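; BP_FunctionTools is a tool Blueprint with one helper that samples a float curve on a repeating timer and remaps the result.
; SmoothlyGetMappedCurveValue advances a caller-held, by-ref elapsed time by delta seconds, wrapping it at the ratio of mapping period to curve period.
; It samples the curve at that time divided by the ratio, then clamp-maps the value from the curve's range to the target range.
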(fn `SmoothlyGetMappedCurveValue`
  (params (CacheElapsedTime :type "Float (double-precision) (by ref)") (Curve :type "CurveFloat Object Reference (by ref)") (DeltaSeconds :type "Float (double-precision)") (CurvePeriod :type "Float (double-precision)" :default 1.0) (MappingCurvePeriod :type "Float (double-precision)" :default 1.0) (CurveMinValue :type "Float (double-precision)") (CurveMaxValue :type "Float (double-precision)" :default 1.0) (MappingMinValue :type "Float (double-precision)") (MappingMaxValue :type "Float (double-precision)" :default 1.0))
  (returns (OutValue :type "Float (double-precision)"))
  (locals (PeriodMultiples :type "Float (double-precision)"))
  (set `local.PeriodMultiples` (/ MappingCurvePeriod CurvePeriod))
  (`|VariableSetRef` (`local.CacheElapsedTime`) (mod (+ (`local.CacheElapsedTime`) (`local.DeltaSeconds`)) (`local.PeriodMultiples`)))
  (return (`KismetMathLibrary.MapRangeClamped` (`CurveFloat.GetFloatValue` (`local.Curve`) (/ (`local.CacheElapsedTime`) (`local.PeriodMultiples`))) (`local.CurveMinValue`) (`local.CurveMaxValue`) (`local.MappingMinValue`) (`local.MappingMaxValue`))))