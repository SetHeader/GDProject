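; GA_FireBolt is a gameplay ability that casts a Fire Bolt projectile toward the point under the mouse.
; After committing, it gets the cursor hit through target data, turns the avatar to face it via CombatInterface and plays the cast montage.
; A montage gameplay event triggers the yaw-only aimed projectile spawn, then a short delay precedes EndAbility, noted as necessary for the projectile to spawn.
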(event `self.K2_ActivateAbility`
  (bind (_hitresult_bblockinghit _hitresult_binitialoverlap _hitresult_time _hitresult_distance _hitresult_location) (`GameplayStatics.BreakHitResult` (`self.HitResult`)))
  (bind (_returnvalue_roll _returnvalue_pitch _returnvalue_yaw) (`KismetMathLibrary.BreakRotator` (`KismetMathLibrary.Conv_VectorToRotator` (- _hitresult_location (`Actor.K2_GetActorLocation` (`self.GetAvatarActorFromActorInfo`))))))
  (bind _returnvalue (`self.K2_CommitAbility`))
  (if _returnvalue
    (bind (_asynctaskproxy _datadatahandle) (`TargetDataUnderMouse.CreateTargetDataUnderMouse`)
      (:`OnValidDataDelegate`
        (bind _output_get (set `self.HitResult` (`AbilitySystemBlueprintLibrary.GetHitResultFromTargetData` _datadatahandle)))
        (bind _ascombat_interface (cast `CombatInterface` (`self.GetAvatarActorFromActorInfo`)))
        (`CombatInterface.UpdateFacingTarget` _ascombat_interface (`.Location` (`GameplayStatics.BreakHitResult` _output_get)))
        (`AbilityTask_PlayMontageAndWait.CreatePlayMontageAndWaitProxy` "None" "/Game/GDContent/Animations/Aura/AM_Cast_FireBolt.AM_Cast_FireBolt" 1.0 "None" false
          (:`then`
            (`AbilityTask_WaitGameplayEvent.WaitGameplayEvent` (struct :`TagName` "Event.Montage.FireBolt") null
              (:`EventReceived`
                (`self.SpawnProjectile` (`KismetMathLibrary.MakeRotator` 0.0 0.0 _returnvalue_yaw))
                ;[1 1 1] 重要！不停止一段时间会导致无法生成发射物
                (`KismetSystemLibrary.Delay` 0.5)
                (`self.K2_EndAbility`)))))))
    (else
      (`self.K2_EndAbility`))))