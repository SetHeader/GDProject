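; FireBolt gameplay ability that casts a projectile toward the point under the mouse.
; After committing, it takes mouse target data, updates the avatar's facing through CombatInterface, draws a debug sphere and plays the cast montage.
; On authority only, the montage's gameplay event triggers a yaw-only projectile spawn toward the hit location, then ends the ability.
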(event `self.K2_ActivateAbility`
  (bind (_hitresult_bblockinghit _hitresult_binitialoverlap _hitresult_time _hitresult_distance _hitresult_location) (`GameplayStatics.BreakHitResult` (`self.HitResult`)))
  (bind (_returnvalue_roll _returnvalue_pitch _returnvalue_yaw) (`KismetMathLibrary.BreakRotator` (`KismetMathLibrary.Conv_VectorToRotator` (- _hitresult_location (`Actor.K2_GetActorLocation` (`self.GetAvatarActorFromActorInfo`))))))
  (bind _returnvalue (`self.K2_CommitAbility`))
  (if _returnvalue
    (bind (_asynctaskproxy _datadatahandle) (`TargetDataUnderMouse.CreateTargetDataUnderMouse`)
      (:`OnValidDataDelegate`
        (bind _output_get (set `self.HitResult` (`AbilitySystemBlueprintLibrary.GetHitResultFromTargetData` _datadatahandle)))
        (bind _ascombat_interface (cast `CombatInterface` (`self.GetAvatarActorFromActorInfo`)))
        (`CombatInterface.UpdateFacingTarget` _ascombat_interface (`.Location` (`GameplayStatics.BreakHitResult` _output_get)))
        (`KismetSystemLibrary.DrawDebugSphere` (`.Location` (`GameplayStatics.BreakHitResult` _output_get)) 20.0 12 (struct :`R` 1.0 :`G` 1.0 :`B` 1.0 :`A` 1.0) 5.0)
        (`AbilityTask_PlayMontageAndWait.CreatePlayMontageAndWaitProxy` "None" "/Game/GDContent/Animations/AM_Cast_FireBolt.AM_Cast_FireBolt" 1.0 "None" false
          (:`then`
            (`self.K2_HasAuthority`
              (:`True`
                (`AbilityTask_WaitGameplayEvent.WaitGameplayEvent` (struct :`TagName` "Event.Montage.FireBolt") null
                  (:`EventReceived`
                    (`self.SpawnProjectile` (`KismetMathLibrary.MakeRotator` 0.0 0.0 _returnvalue_yaw))
                    (`self.K2_EndAbility`)))))))))
    (else
      (`self.K2_EndAbility`))))